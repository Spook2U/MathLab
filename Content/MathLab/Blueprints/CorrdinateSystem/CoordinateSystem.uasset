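; MathLab coordinate system actor that displays 3D axes and geometry elements, with keys to move it vertically and resize its axes.
; Save and Load store display settings and geometry in a MathLabSave slot as typed structs, rebuilding elements through Add functions.
; BeginPlay runs a pausable Timeline demo moving a sphere through a plane, recreating the intersection point or circle every update.
; Line, three-plane and "answer to everything" demos are present but unwired.
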(event EventBeginPlay
  (Utilities|FlowControl|Sequence
    (:then_0
      ;[1 1 1] Enable Keyboard Input
      (Input|EnableInput (Game|GetPlayerController 0)))
    (:then_1
      (CallFunction|Init)
      ;[1 1 1] Units?
      (if true
        (Class|CoordinateSystemBase|AddUnits))
      (Utilities|FlowControl|Sequence
        (:then_0
          (if true ; Necessary, cause Timeline inside
            (|SphereMovesThroughPlane) ; Press P for Pause, C for Continue
          ))))))

(event Input|KeyboardEvents|Up
  (params (Key :type Key%20Structure :default "AnyKey"))
  (bind _defaultsceneroot (Variables|Default|GetDefaultSceneRoot))
  (bind _returnvalue (Transformation|GetWorldLocation _defaultsceneroot))
  ;[1 1 1] Move Coordinate System Up & Down
  (:Pressed
    (Transformation|SetWorldLocation _defaultsceneroot (Math|Vector|MakeVector (.x _returnvalue) (.y _returnvalue) (+ (.z _returnvalue) 2e+01)) false false)
    (Class|CoordinateSystemBase|Update)))

(event Input|KeyboardEvents|Down
  (params (Key :type Key%20Structure :default "AnyKey"))
  (bind _defaultsceneroot (Variables|Default|GetDefaultSceneRoot))
  (bind _returnvalue (Transformation|GetWorldLocation _defaultsceneroot))
  ;[1 1 1] Move Coordinate System Up & Down
  (:Pressed
    (Transformation|SetWorldLocation _defaultsceneroot (Math|Vector|MakeVector (.x _returnvalue) (.y _returnvalue) (- (.z _returnvalue) 2e+01)) false false)
    (Class|CoordinateSystemBase|Update)))

(event Input|KeyboardEvents|L
  (params (Key :type Key%20Structure :default "AnyKey"))
  ;[1 1 1] Save & Load
  (:Pressed
    (Class|CoordinateSystemBase|BpDebugScreen "Load" "(R=1.000000,G=1.000000,B=1.000000,A=1.000000)")
    (CallFunction|Load "Slot1")))

(event Input|KeyboardEvents|O
  (params (Key :type Key%20Structure :default "AnyKey"))
  ;[1 1 1] Save & Load
  (:Pressed
    (Class|CoordinateSystemBase|BpDebugScreen "Save" "(R=1.000000,G=1.000000,B=1.000000,A=1.000000)")
    (CallFunction|Save "Slot1")))

(event Input|KeyboardEvents|+
  (params (Key :type Key%20Structure :default "AnyKey"))
  ;[1 1 1] Scale Coordinate System
  (:Pressed
    (Class|CoordinateSystemBase|ScaleAxis (+ (Variables|Default|GetAxisLength) 0.2) (Variables|Default|GetAxisSize))
    (Class|CoordinateSystemBase|Update)))

(event Input|KeyboardEvents|#
  (params (Key :type Key%20Structure :default "AnyKey"))
  ;[1 1 1] Scale Coordinate System
  (:Pressed
    (Class|CoordinateSystemBase|ScaleAxis (- (Variables|Default|GetAxisLength) 0.2) (Variables|Default|GetAxisSize))
    (Class|CoordinateSystemBase|Update)))

(fn ConstructionScript
  (CallFunction|Init)
  (Class|CoordinateSystemBase|ScaleAxis (Variables|Default|GetAxisLength) (Variables|Default|GetAxisSize)))

(fn Init
  (Class|CoordinateSystemBase|SetComponents (Variables|Default|GetX-Axis) (Variables|Default|GetY-Axis) (Variables|Default|GetZ-Axis) (Variables|Default|GetXArrow) (Variables|Default|GetYArrow) (Variables|Default|GetZArrow) (Variables|Default|GetXName) (Variables|Default|GetYName) (Variables|Default|GetZName)))

(fn Save
  (params (Slot :type String))
  (LocalVariables|SetSaveSlot Slot)
  ;[1 1 1] Create SaveGame Instance
  (bind _returnvalue (SaveGame|CreateSaveGameObject "/Game/MathLab/Blueprints/MathLabSave.MathLabSave_C"))
  (bind _asmath_lab_save (Utilities|Casting|CastToMathLabSave _returnvalue))
  (LocalVariables|SetsaveInstance _asmath_lab_save)
  (Utilities|FlowControl|Sequence
    (:then_0
      ;[1 1 1] Save Coordinate System Data
      (Utilities|FlowControl|Sequence
        (:then_0
          (Variables|/Game/MathLab/Blueprints/MathLabSave.MathLabSave_C|SetaxisLength (LocalVariables|GetsaveInstance) (Variables|Default|GetaxisLength))
          (Variables|/Game/MathLab/Blueprints/MathLabSave.MathLabSave_C|SetaxisSize (LocalVariables|GetsaveInstance) (Variables|Default|GetaxisSize))
          (Variables|/Game/MathLab/Blueprints/MathLabSave.MathLabSave_C|Setglowiness (LocalVariables|GetsaveInstance) (Variables|Default|Getglowiness))
          (Variables|/Game/MathLab/Blueprints/MathLabSave.MathLabSave_C|SetxAxisName (LocalVariables|GetsaveInstance) (Variables|Default|GetxAxisName))
          (Variables|/Game/MathLab/Blueprints/MathLabSave.MathLabSave_C|SetyAxisName (LocalVariables|GetsaveInstance) (Variables|Default|GetyAxisName))
          (Variables|/Game/MathLab/Blueprints/MathLabSave.MathLabSave_C|SetzAxisName (LocalVariables|GetsaveInstance) (Variables|Default|GetzAxisName)))
        (:then_1
          (Variables|/Game/MathLab/Blueprints/MathLabSave.MathLabSave_C|SetshowUnitLaser (LocalVariables|GetsaveInstance) (Variables|Default|GetshowUnitLaser))
          (Variables|/Game/MathLab/Blueprints/MathLabSave.MathLabSave_C|SetunitCount (LocalVariables|GetsaveInstance) (Variables|Default|GetunitCount))
          (Variables|/Game/MathLab/Blueprints/MathLabSave.MathLabSave_C|SetunitLaserColor (LocalVariables|GetsaveInstance) (Variables|Default|GetunitLaserColor))
          (Variables|/Game/MathLab/Blueprints/MathLabSave.MathLabSave_C|SetunitGlowiness (LocalVariables|GetsaveInstance) (Variables|Default|GetunitGlowiness))
          (Variables|/Game/MathLab/Blueprints/MathLabSave.MathLabSave_C|SetunitSizeFactor (LocalVariables|GetsaveInstance) (Variables|Default|GetunitSizeFactor))
          (Variables|/Game/MathLab/Blueprints/MathLabSave.MathLabSave_C|SetunitLaserSizeFactor (LocalVariables|GetsaveInstance) (Variables|Default|GetunitLaserSizeFactor)))
        (:then_2
          (Variables|/Game/MathLab/Blueprints/MathLabSave.MathLabSave_C|SetshowNames (LocalVariables|GetsaveInstance) (Variables|Default|GetshowNames))
          (Variables|/Game/MathLab/Blueprints/MathLabSave.MathLabSave_C|SetshowMathData (LocalVariables|GetsaveInstance) (Variables|Default|GetshowMathData))
          (Variables|/Game/MathLab/Blueprints/MathLabSave.MathLabSave_C|SetnameTextSize (LocalVariables|GetsaveInstance) (Variables|Default|GetnameTextSize))
          (Variables|/Game/MathLab/Blueprints/MathLabSave.MathLabSave_C|SetunitTextSize (LocalVariables|GetsaveInstance) (Variables|Default|GetunitTextSize))
          (Variables|/Game/MathLab/Blueprints/MathLabSave.MathLabSave_C|SetaxisTextSize (LocalVariables|GetsaveInstance) (Variables|Default|GetaxisTextSize)))
        (:then_3
          (Variables|/Game/MathLab/Blueprints/MathLabSave.MathLabSave_C|SetshowCVectorName (LocalVariables|GetsaveInstance) (Variables|Default|GetshowCVectorName))
          (Variables|/Game/MathLab/Blueprints/MathLabSave.MathLabSave_C|SetshowCVectorMathData (LocalVariables|GetsaveInstance) (Variables|Default|GetshowCVectorMathData)))))
    (:then_1
      ;[1 1 1] Save Geometry Objects
      (Utilities|FlowControl|Sequence
        (:then_0
          (for _array_element (Variables|Default|Getelements)
            (bind _output_get (LocalVariables|Setelement _array_element))
            (switch Utilities|FlowControl|Switch|SwitchonGeometryType (Variables|/Script/MathLab.GeometryBase|Gettype _output_get)
              (:circle
                (bind _ascircle (Utilities|Casting|CastToCircle (LocalVariables|Getelement)))
                (bind _returnvalue_2 (Class|GeometryBase|GetName _ascircle))
                (Utilities|Array|Add (LocalVariables|GetgeometrySave) (Utilities|Struct|MakeGeometrySaveData "circle" (Variables|/Script/MathLab.GeometryBase|Getcolor _ascircle) "(coordinate=(X=0.000000,Y=0.000000,Z=0.000000))" "(position=(X=0.000000,Y=0.000000,Z=0.000000),direction=(X=0.000000,Y=0.000000,Z=0.000000))" "(position=(X=0.000000,Y=0.000000,Z=0.000000),direction1=(X=0.000000,Y=0.000000,Z=0.000000),direction2=(X=0.000000,Y=0.000000,Z=0.000000))" "(center=(X=0.000000,Y=0.000000,Z=0.000000),radius=0.000000)" (Variables|/Script/MathLab.CircleBase|Getcircle _ascircle) _returnvalue_2 (Variables|/Script/MathLab.GeometryBase|GetshowConstruction _ascircle))))
              (:line
                (bind _asline (Utilities|Casting|CastToLine (LocalVariables|Getelement)))
                (bind _returnvalue_3 (Class|GeometryBase|GetName _asline))
                (Utilities|Array|Add (LocalVariables|GetgeometrySave) (Utilities|Struct|MakeGeometrySaveData "line" (Variables|/Script/MathLab.GeometryBase|Getcolor _asline) "(coordinate=(X=0.000000,Y=0.000000,Z=0.000000))" (Variables|/Script/MathLab.LineBase|Getline _asline) "(position=(X=0.000000,Y=0.000000,Z=0.000000),direction1=(X=0.000000,Y=0.000000,Z=0.000000),direction2=(X=0.000000,Y=0.000000,Z=0.000000))" "(center=(X=0.000000,Y=0.000000,Z=0.000000),radius=0.000000)" "(center=(X=0.000000,Y=0.000000,Z=0.000000),normal=(X=0.000000,Y=0.000000,Z=0.000000),radius=0.000000)" _returnvalue_3 (Variables|/Script/MathLab.GeometryBase|GetshowConstruction _asline))))
              (:plane
                (bind _asplane (Utilities|Casting|CastToPlane (LocalVariables|Getelement)))
                (bind _returnvalue_4 (Class|GeometryBase|GetName _asplane))
                (Utilities|Array|Add (LocalVariables|GetgeometrySave) (Utilities|Struct|MakeGeometrySaveData "plane" (Variables|/Script/MathLab.GeometryBase|Getcolor _asplane) "(coordinate=(X=0.000000,Y=0.000000,Z=0.000000))" "(position=(X=0.000000,Y=0.000000,Z=0.000000),direction=(X=0.000000,Y=0.000000,Z=0.000000))" (Variables|/Script/MathLab.PlaneBase|Getplane _asplane) "(center=(X=0.000000,Y=0.000000,Z=0.000000),radius=0.000000)" "(center=(X=0.000000,Y=0.000000,Z=0.000000),normal=(X=0.000000,Y=0.000000,Z=0.000000),radius=0.000000)" _returnvalue_4 (Variables|/Script/MathLab.GeometryBase|GetshowConstruction _asplane))))
              (:point
                (bind _aspoint (Utilities|Casting|CastToPoint (LocalVariables|Getelement)))
                (bind _returnvalue_5 (Class|GeometryBase|GetName _aspoint))
                (Utilities|Array|Add (LocalVariables|GetgeometrySave) (Utilities|Struct|MakeGeometrySaveData "point" (Variables|/Script/MathLab.GeometryBase|Getcolor _aspoint) (Variables|/Script/MathLab.PointBase|Getpoint _aspoint) "(position=(X=0.000000,Y=0.000000,Z=0.000000),direction=(X=0.000000,Y=0.000000,Z=0.000000))" "(position=(X=0.000000,Y=0.000000,Z=0.000000),direction1=(X=0.000000,Y=0.000000,Z=0.000000),direction2=(X=0.000000,Y=0.000000,Z=0.000000))" "(center=(X=0.000000,Y=0.000000,Z=0.000000),radius=0.000000)" "(center=(X=0.000000,Y=0.000000,Z=0.000000),normal=(X=0.000000,Y=0.000000,Z=0.000000),radius=0.000000)" _returnvalue_5 (Variables|/Script/MathLab.GeometryBase|GetshowConstruction _aspoint))))
              (:sphere
                (bind _assphere (Utilities|Casting|CastToSphere (LocalVariables|Getelement)))
                (bind _returnvalue_6 (Class|GeometryBase|GetName _assphere))
                (Utilities|Array|Add (LocalVariables|GetgeometrySave) (Utilities|Struct|MakeGeometrySaveData "sphere" (Variables|/Script/MathLab.GeometryBase|Getcolor _assphere) "(coordinate=(X=0.000000,Y=0.000000,Z=0.000000))" "(position=(X=0.000000,Y=0.000000,Z=0.000000),direction=(X=0.000000,Y=0.000000,Z=0.000000))" "(position=(X=0.000000,Y=0.000000,Z=0.000000),direction1=(X=0.000000,Y=0.000000,Z=0.000000),direction2=(X=0.000000,Y=0.000000,Z=0.000000))" (Variables|/Script/MathLab.SphereBase|Getsphere _assphere) "(center=(X=0.000000,Y=0.000000,Z=0.000000),normal=(X=0.000000,Y=0.000000,Z=0.000000),radius=0.000000)" _returnvalue_6 (Variables|/Script/MathLab.GeometryBase|GetshowConstruction _assphere)))))))
        (:then_1
          (Variables|/Game/MathLab/Blueprints/MathLabSave.MathLabSave_C|Setelements (LocalVariables|GetsaveInstance) (LocalVariables|GetgeometrySave)))))
    (:then_2
      ;[1 1 1] Save Game
      (SaveGame|SaveGametoSlot (LocalVariables|GetsaveInstance) (LocalVariables|GetSaveSlot)))))

(fn Load
  (params (Slot :type String))
  ;[1 1 1] Load SaveGame Instance
  (bind _returnvalue (SaveGame|LoadGamefromSlot Slot))
  (bind _asmath_lab_save (Utilities|Casting|CastToMathLabSave _returnvalue))
  (LocalVariables|SetsaveInstance _asmath_lab_save)
  (Utilities|FlowControl|Sequence
    (:then_0
      ;[1 1 1] Load Coordinate System Data
      (Utilities|FlowControl|Sequence
        (:then_0
          (Variables|Default|SetaxisLength (Variables|/Game/MathLab/Blueprints/MathLabSave.MathLabSave_C|GetaxisLength (LocalVariables|GetsaveInstance)))
          (Variables|Default|SetaxisSize (Variables|/Game/MathLab/Blueprints/MathLabSave.MathLabSave_C|GetaxisSize (LocalVariables|GetsaveInstance)))
          (Variables|Default|Setglowiness (Variables|/Game/MathLab/Blueprints/MathLabSave.MathLabSave_C|Getglowiness (LocalVariables|GetsaveInstance)))
          (Variables|Default|SetxAxisName (Variables|/Game/MathLab/Blueprints/MathLabSave.MathLabSave_C|GetxAxisName (LocalVariables|GetsaveInstance)))
          (Variables|Default|SetyAxisName (Variables|/Game/MathLab/Blueprints/MathLabSave.MathLabSave_C|GetyAxisName (LocalVariables|GetsaveInstance)))
          (Variables|Default|SetzAxisName (Variables|/Game/MathLab/Blueprints/MathLabSave.MathLabSave_C|GetzAxisName (LocalVariables|GetsaveInstance))))
        (:then_1
          (Variables|Default|SetshowUnitLaser (Variables|/Game/MathLab/Blueprints/MathLabSave.MathLabSave_C|GetshowUnitLaser (LocalVariables|GetsaveInstance)))
          (Variables|Default|SetunitCount (Variables|/Game/MathLab/Blueprints/MathLabSave.MathLabSave_C|GetunitCount (LocalVariables|GetsaveInstance)))
          (Variables|Default|SetunitLaserColor (Variables|/Game/MathLab/Blueprints/MathLabSave.MathLabSave_C|GetunitLaserColor (LocalVariables|GetsaveInstance)))
          (Variables|Default|Setglowiness (Variables|/Game/MathLab/Blueprints/MathLabSave.MathLabSave_C|GetunitGlowiness (LocalVariables|GetsaveInstance)))
          (Variables|Default|SetunitSizeFactor (Variables|/Game/MathLab/Blueprints/MathLabSave.MathLabSave_C|GetunitSizeFactor (LocalVariables|GetsaveInstance)))
          (Variables|Default|SetunitLaserSizeFactor (Variables|/Game/MathLab/Blueprints/MathLabSave.MathLabSave_C|GetunitLaserSizeFactor (LocalVariables|GetsaveInstance))))
        (:then_2
          (Variables|Default|SetshowNames (Variables|/Game/MathLab/Blueprints/MathLabSave.MathLabSave_C|GetshowNames (LocalVariables|GetsaveInstance)))
          (Variables|Default|SetshowMathData (Variables|/Game/MathLab/Blueprints/MathLabSave.MathLabSave_C|GetshowMathData (LocalVariables|GetsaveInstance)))
          (Variables|Default|SetnameTextSize (Variables|/Game/MathLab/Blueprints/MathLabSave.MathLabSave_C|GetnameTextSize (LocalVariables|GetsaveInstance)))
          (Variables|Default|SetunitTextSize (Variables|/Game/MathLab/Blueprints/MathLabSave.MathLabSave_C|GetunitTextSize (LocalVariables|GetsaveInstance)))
          (Variables|Default|SetaxisTextSize (Variables|/Game/MathLab/Blueprints/MathLabSave.MathLabSave_C|GetaxisTextSize (LocalVariables|GetsaveInstance))))
        (:then_3
          (Variables|Default|SetshowCVectorName (Variables|/Game/MathLab/Blueprints/MathLabSave.MathLabSave_C|GetshowCVectorName (LocalVariables|GetsaveInstance)))
          (Variables|Default|SetshowCVectorMathData (Variables|/Game/MathLab/Blueprints/MathLabSave.MathLabSave_C|GetshowCVectorMathData (LocalVariables|GetsaveInstance)))
          (Variables|Default|SetcVectorTextSize (Variables|/Game/MathLab/Blueprints/MathLabSave.MathLabSave_C|GetcVectorTextSize (LocalVariables|GetsaveInstance))))))
    (:then_1
      ;[1 1 1] Load Geometry Objects
      (for _array_element (Variables|/Game/MathLab/Blueprints/MathLabSave.MathLabSave_C|Getelements (LocalVariables|GetsaveInstance))
        (bind _output_get (LocalVariables|SetelementStruct _array_element))
        (switch Utilities|FlowControl|Switch|SwitchonGeometryType (.type (Utilities|Struct|BreakGeometrySaveData _output_get))
          (:circle
            (Class|CoordinateSystemBase|AddCircle (.color (Utilities|Struct|BreakGeometrySaveData (LocalVariables|GetelementStruct))) (.circle (Utilities|Struct|BreakGeometrySaveData (LocalVariables|GetelementStruct))) (.name (Utilities|Struct|BreakGeometrySaveData (LocalVariables|GetelementStruct))) (.showConstruction (Utilities|Struct|BreakGeometrySaveData (LocalVariables|GetelementStruct)))))
          (:line
            (Class|CoordinateSystemBase|AddLine (.color (Utilities|Struct|BreakGeometrySaveData (LocalVariables|GetelementStruct))) (.line (Utilities|Struct|BreakGeometrySaveData (LocalVariables|GetelementStruct))) (.lineMode (Utilities|Struct|BreakGeometrySaveData (LocalVariables|GetelementStruct))) (.name (Utilities|Struct|BreakGeometrySaveData (LocalVariables|GetelementStruct))) (.showConstruction (Utilities|Struct|BreakGeometrySaveData (LocalVariables|GetelementStruct)))))
          (:plane
            (Class|CoordinateSystemBase|AddPlane (.color (Utilities|Struct|BreakGeometrySaveData (LocalVariables|GetelementStruct))) (.plane (Utilities|Struct|BreakGeometrySaveData (LocalVariables|GetelementStruct))) "plane" (.name (Utilities|Struct|BreakGeometrySaveData (LocalVariables|GetelementStruct))) (.showConstruction (Utilities|Struct|BreakGeometrySaveData (LocalVariables|GetelementStruct)))))
          (:point
            (Class|CoordinateSystemBase|AddPoint (.color (Utilities|Struct|BreakGeometrySaveData (LocalVariables|GetelementStruct))) (.point (Utilities|Struct|BreakGeometrySaveData (LocalVariables|GetelementStruct))) (.name (Utilities|Struct|BreakGeometrySaveData (LocalVariables|GetelementStruct))) (.showConstruction (Utilities|Struct|BreakGeometrySaveData (LocalVariables|GetelementStruct)))))
          (:sphere
            (Class|CoordinateSystemBase|AddSphere (.color (Utilities|Struct|BreakGeometrySaveData (LocalVariables|GetelementStruct))) (.sphere (Utilities|Struct|BreakGeometrySaveData (LocalVariables|GetelementStruct))) (.name (Utilities|Struct|BreakGeometrySaveData (LocalVariables|GetelementStruct))) (.showConstruction (Utilities|Struct|BreakGeometrySaveData (LocalVariables|GetelementStruct))))))))
    (:then_2
      (Class|CoordinateSystemBase|Update))))

(event Input|KeyboardEvents|P
  (params (Key :type Key%20Structure :default "AnyKey"))
  (:Pressed
    (bind _sphere_movement (Timeline|Sphere%20Movement Stop)
      (:Update
        (Class|SphereBase|SetSphere (stale _returnvalue) (Utilities|Struct|MakeMathSphere (Math|Vector|MakeVector (.x (.center (Class|CoordinateSystemBase|SphereBPtoFSphere (stale _returnvalue)))) _sphere_movement (.z (.center (Class|CoordinateSystemBase|SphereBPtoFSphere (stale _returnvalue))))) (.radius (Class|CoordinateSystemBase|SphereBPtoFSphere (stale _returnvalue)))))
        (bind _returnvalue (Class|CoordinateSystemBase|GetRelativePosition (stale _returnvalue) (stale _returnvalue)))
        (bind (_found _returnvalue_2) (Class|CoordinateSystemBase|FindGeometrywithName "Intersection"))
        (if _found
          (Class|CoordinateSystemBase|Remove _returnvalue_2))
        (switch Utilities|FlowControl|Switch|SwitchonRelation (.relation _returnvalue)
          (:intersection
            (switch Utilities|FlowControl|Switch|SwitchonIntersectionType (.type (.intersections _returnvalue))
              (:point
                (bind _returnvalue_3 (Class|CoordinateSystemBase|AddPoint "white" (.point (.intersections _returnvalue)) "Intersection" false))
                (Class|GeometryBase|SetupName _returnvalue_3 false false false false))
              (:circle
                (bind _returnvalue_4 (Class|CoordinateSystemBase|AddCircle "white" (.circle (.intersections _returnvalue)) "Intersection" false))
                (Class|GeometryBase|SetupName _returnvalue_4 false false false false)))))))))

(event Input|KeyboardEvents|C
  (params (Key :type Key%20Structure :default "AnyKey"))
  (:Pressed
    (bind _sphere_movement (Timeline|Sphere%20Movement Play)
      (:Update
        (Class|SphereBase|SetSphere (stale _returnvalue) (Utilities|Struct|MakeMathSphere (Math|Vector|MakeVector (.x (.center (Class|CoordinateSystemBase|SphereBPtoFSphere (stale _returnvalue)))) _sphere_movement (.z (.center (Class|CoordinateSystemBase|SphereBPtoFSphere (stale _returnvalue))))) (.radius (Class|CoordinateSystemBase|SphereBPtoFSphere (stale _returnvalue)))))
        (bind _returnvalue (Class|CoordinateSystemBase|GetRelativePosition (stale _returnvalue) (stale _returnvalue)))
        (bind (_found _returnvalue_2) (Class|CoordinateSystemBase|FindGeometrywithName "Intersection"))
        (if _found
          (Class|CoordinateSystemBase|Remove _returnvalue_2))
        (switch Utilities|FlowControl|Switch|SwitchonRelation (.relation _returnvalue)
          (:intersection
            (switch Utilities|FlowControl|Switch|SwitchonIntersectionType (.type (.intersections _returnvalue))
              (:point
                (bind _returnvalue_3 (Class|CoordinateSystemBase|AddPoint "white" (.point (.intersections _returnvalue)) "Intersection" false))
                (Class|GeometryBase|SetupName _returnvalue_3 false false false false))
              (:circle
                (bind _returnvalue_4 (Class|CoordinateSystemBase|AddCircle "white" (.circle (.intersections _returnvalue)) "Intersection" false))
                (Class|GeometryBase|SetupName _returnvalue_4 false false false false)))))))))